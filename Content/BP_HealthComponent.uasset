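; BP_HealthComponent is a health component that stores a Health value, exposed through a getter.
; On BeginPlay it binds a handler to its OnHealthChanged dispatcher, which sums the delta and Health, then calls the UpdateProgressBar dispatcher.
; The clamp ignores that sum and has all inputs at zero, so every change sets Health to zero.
; Unconnected nodes for broadcasting OnHealthChanged and binding UpdateProgressBar never run.
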(event Custom|OnHealthChanged_Event
  (params (Delta :type Float%20%28double-precision%29))
  (Variables|Default|SetNewVar (+ Delta (Variables|Default|GetHealth)))
  (Variables|Default|SetHealth (Math|Conversions|ToFloat(Integer) (Math|Integer|Clamp(Integer) 0 0 0)))
  (Default|CallUpdateProgressBar))

(event EventBeginPlay
  (EventDispatchers|BindEventtoOnHealthChanged (EventDispatchers|CreateEvent :!event Custom|OnHealthChanged_Event)))

(fn GetFunction
  (return (Variables|Default|GetHealth)))
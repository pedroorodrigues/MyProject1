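; Door actor that swings open and closed when triggered while something overlaps its box.
; Box overlap sets a collision flag and adds a prompt widget to the viewport, removing it on exit.
; BeginPlay binds an event to a dispatcher after casting to the custom player controller.
; The toggle event plays a timeline forward or in reverse to drive the mesh's relative yaw, flipping the open state when finished.
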(event OnComponentBeginOverlap(Box)
  (params (OverlappedComponent :type Primitive%20Component%20Object%20Reference) (OtherActor :type Actor%20Object%20Reference) (OtherComp :type Primitive%20Component%20Object%20Reference) (OtherBodyIndex :type Integer) (bFromSweep :type Boolean) (SweepResult :type Hit%20Result%20Structure%20%28by%20ref%29))
  (Variables|Default|SetonCollision true)
  (bind _returnvalue (UserInterface|CreateWidget "/Game/wigets/weitget.weitget_C"))
  (bind _output_get (Variables|Default|SetNewVar _returnvalue))
  (UserInterface|Viewport|AddtoViewport _output_get 0))

(event OnComponentEndOverlap(Box)
  (params (OverlappedComponent :type Primitive%20Component%20Object%20Reference) (OtherActor :type Actor%20Object%20Reference) (OtherComp :type Primitive%20Component%20Object%20Reference) (OtherBodyIndex :type Integer))
  (Variables|Default|SetonCollision false)
  (Widget|RemovefromParent (Variables|Default|GetNewVar)))

(event Custom|CustomEvent)

(event EventNewFunction
  (bind _returnvalue (Transformation|GetActorRotation))
  (bind (_roll _pitch) (Math|Rotator|BreakRotator _returnvalue))
  (if (Variables|Default|GetonCollision)
    (if (Variables|Default|GetisOpen)
      (bind _newtrack_0 (Timeline|My%20Timelie ReverseFromEnd)
        (:Update
          (Transformation|SetRelativeRotation (Variables|Default|GetStaticMesh) (Math|Rotator|MakeRotator _roll _pitch _newtrack_0) false false))
        (:Finished
          (Variables|Default|SetisOpen (not (Variables|Default|GetisOpen)))))
      (else
        (Timeline|My%20Timelie PlayFromStart)))))

(event EventBeginPlay
  (Utilities|Casting|CastToplayercontroller (Game|GetPlayerController 0))
  (EventDispatchers|BindEventtoNewEventDispatcher (EventDispatchers|CreateEvent :!event Custom|CustomEvent)))

(fn ConstructionScript)
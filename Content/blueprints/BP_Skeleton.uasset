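; BP_Skeleton is an enemy that chases the player character and is destroyed by any damage.
; Every Tick it reads the player's location, then re-issues AI MoveTo with the player as target, caching the character reference in that move step.
; Tick also feeds Health into a world-space health bar widget and rotates it to face the camera.
; The damage event destroys the actor outright without changing Health.
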(event Custom|move%20towerds%20to%20player
  (bind _asbp_third_person_character (Utilities|Casting|CastToBP_ThirdPersonCharacter (Game|GetPlayerCharacter 0)))
  (bind _output_get (Variables|Default|SetAs%20BP%20Third%20Person%20Character _asbp_third_person_character))
  (AI|AIMoveTo self (Variables|Default|GetPlayer%20POS) _output_get 1e+02 false))

(event Custom|Get%20Player%20Position
  (Variables|Default|SetPlayer%20POS (Transformation|GetActorLocation (Variables|Default|GetAs%20BP%20Third%20Person%20Character))))

(event Game|Damage|EventAnyDamage
  (params (Damage :type Float%20%28single-precision%29) (DamageType :type Damage%20Type%20Object%20Reference) (InstigatedBy :type Controller%20Object%20Reference) (DamageCauser :type Actor%20Object%20Reference))
  (Actor|DestroyActor))

(event EventTick
  (params (DeltaSeconds :type Float%20%28single-precision%29))
  (CallFunction|GetPlayerPosition)
  (CallFunction|MoveTowerdstoPlayer)
  (bind _aswb_enemy_health_bar (Utilities|Casting|CastToWB_EnemyHealthBar (UserInterface|GetWidget (Variables|Default|GetHealthBarWidget))))
  (Progress|SetPercent (Variables|/Game/WB_EnemyHealthBar.WB_EnemyHealthBar_C|GetHealthBar _aswb_enemy_health_bar) (/ (Variables|Default|Gethealth) 1e+02))
  (Transformation|SetWorldRotation (Variables|Default|GetHealthBarWidget) (Math|Rotator|FindLookatRotation (Transformation|GetWorldLocation (Variables|Default|GetHealthBarWidget)) (Transformation|GetWorldLocation (Variables|/Script/Engine.PlayerCameraManager|GetTransformComponent (Game|GetPlayerCameraManager 0)))) false false))

(event EventBeginPlay)

(fn ConstructionScript)